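; BP_Bullet is a bullet actor that damages a StarshipCharacter it overlaps.
; The collision box's begin-overlap event ignores other actors, stores the ship reference and calls DamagePlayer.
; DamagePlayer applies fixed damage, spawns an explosion emitter at the ship's mesh location and destroys the bullet.
; The graph contains no movement logic, and the construction script is empty.
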(event OnComponentBeginOverlap(CollsionBox)
  (params (OverlappedComponent :type Primitive%20Component%20Object%20Reference) (OtherActor :type Actor%20Object%20Reference) (OtherComp :type Primitive%20Component%20Object%20Reference) (OtherBodyIndex :type Integer) (bFromSweep :type Boolean) (SweepResult :type Hit%20Result%20Structure%20%28by%20ref%29))
  (bind _asstarship_character (Utilities|Casting|CastToStarshipCharacter OtherActor))
  (Variables|Default|SetAs%20Starship%20Character _asstarship_character)
  (CallFunction|DamagePlayer))

(event Custom|DamagePlayer
  ;[1 1 1] Damage Player
  (Game|Damage|ApplyDamage (Variables|Default|GetAs%20Starship%20Character) 1e+01 0 0)
  (Effects|SpawnEmitteratLocation "/Game/FXVarietyPack/Particles/P_ky_explosion.P_ky_explosion" (Transformation|GetWorldLocation (Variables|/Script/Engine.Character|GetMesh (Variables|Default|GetAs%20Starship%20Character))))
  (Actor|DestroyActor))

(fn ConstructionScript)