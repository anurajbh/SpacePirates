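; BP_ChaseShip is an AI enemy ship that turns toward and fires at the player's starship.
; AI Perception updates write spotted state and location to the Blackboard and toggle CanShoot.
; A Delay on Tick gates firing to roughly two-second intervals, aiming an arrow at the player to spawn BP_Bullet.
; Self-recursive Delay loops check range and smoothly rotate the ship toward the player when within 1000 units.
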(event OnPerceptionUpdated(AIPerception)
  (params (UpdatedActors :type Array%20of%20Actor%20Object%20References))
  (bind _returnvalue (AI|GetBlackboard 0))
  ;[1 1 1] Update BB Value
  (for _array_element UpdatedActors
    (bind _info (Class|AIPerceptionComponent|GetActorsPerception (Variables|Default|GetAIPerception) _array_element))
    (for (_array_element_2 _array_index) (.LastSensedStimuli (Utilities|Struct|BreakActorPerceptionBlueprintInfo _info))
      (Development|PrintString (Utilities|String|Append (Utilities|String|ToString(Integer) _array_index) (Utilities|String|ToString(Boolean) (.bSuccessfullySensed (Utilities|Struct|BreakAIStimulus _array_element_2)))) true true "(R=0.000000,G=0.660000,B=1.000000,A=1.000000)" 5.0)
      (if (.bSuccessfullySensed (Utilities|Struct|BreakAIStimulus _array_element_2))
        (AI|Components|Blackboard|SetValueasBool _returnvalue (Utilities|Name|MakeLiteralName "SpaceShipSpotted") true)
        (AI|Components|Blackboard|SetValueasVector _returnvalue (Utilities|Name|MakeLiteralName "SpaceShipLocation") (.StimulusLocation (Utilities|Struct|BreakAIStimulus _array_element_2)))
        ;[1 1 1] Can Shoot Bool
        (Variables|Default|SetCanShoot true)
        (Development|PrintString "CanShoot True")
        (else
          (AI|Components|Blackboard|SetValueasBool (AI|GetBlackboard 0) (Utilities|Name|MakeLiteralName "SpaceShipSpotted") false)
          (Variables|Default|SetCanShoot false)
          (Development|PrintString "CanShoot False"))))))

(event Custom|Face%20Player
  (bind _returnvalue (Utilities|Time|GetWorldDeltaSeconds))
  (bind _returnvalue_2 (Transformation|GetActorLocation))
  (bind _returnvalue_3 (Transformation|GetActorRotation))
  (bind _as_starship_character (Variables|Default|GetAs%20Starship%20Character))
  (bind _returnvalue_4 (Transformation|GetActorLocation _as_starship_character))
  (bind _returnvalue_5 (Math|Rotator|FindLookatRotation _returnvalue_2 _returnvalue_4))
  (bind _returnvalue_6 (Math|Interpolation|RInterpTo _returnvalue_3 _returnvalue_5 _returnvalue 2.0))
  ;[1 1 1] Face Player
  (if (Variables|Default|GetShouldRotate)
    (Transformation|SetActorRotation (Math|Rotator|MakeRotator (.roll _returnvalue_6) (.pitch _returnvalue_6) (.yaw _returnvalue_6)))
    (Utilities|FlowControl|Delay 0.001)
    (CallFunction|FacePlayer)))

(event Custom|Should%20Rotate%20Event
  ;[1 1 1] Should Rotate
  (if (<= (Transformation|GetDistanceTo (Variables|Default|GetAs%20Starship%20Character)) 1e+03)
    (Variables|Default|SetShouldRotate true)
    (CallFunction|FacePlayer)
    (else
      (Variables|Default|SetShouldRotate false)))
  (Utilities|FlowControl|Delay 0.001)
  (CallFunction|ShouldRotateEvent))

(event Custom|ShootAtSpaceship
  (bind _arrow1 (Variables|Default|GetArrow1))
  ;[1 1 1] Shoot At Spaceship
  (Transformation|SetWorldRotation _arrow1 (Math|Rotator|FindLookatRotation (Transformation|GetWorldLocation _arrow1) (Transformation|GetWorldLocation (Variables|/Script/Engine.Actor|GetRootComponent (Game|Player|GetPlayerPawn 0)))) false false)
  (Game|SpawnActorfromClass "/Game/AISpacePatrol/BP_Bullet.BP_Bullet_C" (Transformation|GetWorldTransform (Variables|Default|GetArrow1)) "Undefined" 0 0))

(event EventTick
  (params (DeltaSeconds :type Float%20%28single-precision%29))
  (Utilities|FlowControl|Delay 2.0)
  (if (Variables|Default|GetCanShoot)
    (Development|PrintString "In Shoot Range")
    (CallFunction|ShootatSpaceship)
    (else
      (Development|PrintString "Out of Shoot Range"))))

(event EventBeginPlay
  (bind _asstarship_character (Utilities|Casting|CastToStarshipCharacter (Game|GetPlayerCharacter 0)))
  (Variables|Default|SetAs%20Starship%20Character _asstarship_character)
  (CallFunction|ShouldRotateEvent))

(fn ConstructionScript)