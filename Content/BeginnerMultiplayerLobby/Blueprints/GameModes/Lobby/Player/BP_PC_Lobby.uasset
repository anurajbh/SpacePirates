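; Lobby player controller that handles ready-up interaction and lobby widget toggles.
; On BeginPlay the local controller caches the lobby HUD, which input actions use to toggle the player list and character select.
; A client event shows or hides the ready-up interaction indicator.
; Interact input calls a server event that messages the interact actor, if valid, and flips the Ready flag in the lobby PlayerState.
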(event Custom|SR_Interact
  ;[0.05098 0.05098 0.05098] Ready Up Button Interaction Event which also toggles the Player's ready status
  (bind _interact_actor (Variables|Default|GetInteract_Actor)
    (:then
      (Class|BPINTInteraction|Interact(Message) _interact_actor)
      (CallFunction|ToggleReadyStatus))
    (:else)))

(event Custom|Toggle_ReadyStatus
  ;[0.05098 0.05098 0.05098] Ready Up Button Interaction Event which also toggles the Player's ready status
  ;;[0.05098 0.05098 0.05098] Toggle Ready Status inside the player's PlayerState
  (bind _asbp_ps_lobby (Utilities|Casting|CastToBP_PS_Lobby (Variables|Default|GetPlayerState)))
  (Variables|/Game/BeginnerMultiplayerLobby/Blueprints/GameModes/Lobby/Player/BP_PS_Lobby.BP_PS_Lobby_C|SetReady? _asbp_ps_lobby (not (Variables|/Game/BeginnerMultiplayerLobby/Blueprints/GameModes/Lobby/Player/BP_PS_Lobby.BP_PS_Lobby_C|GetReady? _asbp_ps_lobby))))

(event Custom|OC_Set_ReadyUpIndicator
  (params (CanInteract? :type Boolean))
  (bind _bp_hud_lobby (Variables|Default|GetBP_HUD_Lobby))
  (bind _wb_hud_lobby (Variables|/Game/BeginnerMultiplayerLobby/Blueprints/GameModes/Lobby/Player/BP_HUD_Lobby.BP_HUD_Lobby_C|GetWB_HUD_Lobby _bp_hud_lobby))
  (bind _wb_interactionindicator (Variables|/Game/BeginnerMultiplayerLobby/Widgets/Gameplay/Lobby/WB_HUD_Lobby.WB_HUD_Lobby_C|GetWB_InteractionIndicator _wb_hud_lobby))
  ;[0.05098 0.05098 0.05098] Set ReadyUp Indicator Visiblity (Called by BP_ReadyUpStation)
  (if CanInteract?
    (Widget|SetVisibility _wb_interactionindicator "Visible")
    (else
      (Widget|SetVisibility _wb_interactionindicator "Collapsed"))))

(event EventBeginPlay
  (|CallParentFunction)
  ;[0.05098 0.05098 0.05098] Setup BP_HUD_Lobby reference
  (if (Pawn|IsLocalPlayerController)
    (bind _asbp_hud_lobby (Utilities|GetBPHUDLobby 1e+01)
      (:Success
        (Variables|Default|SetBP_HUD_Lobby _asbp_hud_lobby)))))

(event Input|ActionEvents|InputActionToggle_PlayerList
  (params (Key :type Key%20Structure))
  ;[0.05098 0.05098 0.05098] Toggle Widgets
  (:Pressed
    (Default|TogglePlayerList (Variables|Default|GetBP_HUD_Lobby))))

(event Input|ActionEvents|InputActionInteract
  (params (Key :type Key%20Structure))
  ;[0.05098 0.05098 0.05098] Ready Up Button Interaction Event which also toggles the Player's ready status
  (:Pressed
    (CallFunction|SRInteract)))

(event Input|ActionEvents|InputActionToggle_CharacterSelect
  (params (Key :type Key%20Structure))
  ;[0.05098 0.05098 0.05098] Toggle Widgets
  (:Pressed
    (Default|ToggleCharacterSelect (Variables|Default|GetBP_HUD_Lobby))))

(fn ConstructionScript
  (|CallParentFunction))